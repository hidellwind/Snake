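; Bp_EatGenerator spawns food and pickup actors at random X/Y positions within a square play area at a fixed height.
; On BeginPlay it spawns one Bp_Eat and binds to its OnDestroyed event, so a replacement appears whenever the food is destroyed.
; Two looping timers independently spawn Bp_Haste pickups frequently and Bp_Teleportator actors at a much longer interval, with no cap on their count.
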(event Custom|Spawn%20Eat
  (bind _returnvalue (Game|SpawnActorfromClass "/Game/MyBp/Bp_Eat.Bp_Eat_C" (Math|Transform|MakeTransform (Math|Vector|MakeVector (Math|Random|RandomFloatinRange -1.35e+03 1.35e+03) (Math|Random|RandomFloatinRange -1.35e+03 1.35e+03) -1e+02) "0, 0, 0" "1.000000,1.000000,1.000000") "Undefined" 0 0))
  (Game|BindEventtoOnDestroyed _returnvalue (delegate Custom|EatDestroyed)))

(event Custom|Spawn%20Haste
  (Game|SpawnActorfromClass "/Game/MyBp/Bp_Haste.Bp_Haste_C" (Math|Transform|MakeTransform (Math|Vector|MakeVector (Math|Random|RandomFloatinRange -1.35e+03 1.35e+03) (Math|Random|RandomFloatinRange -1.35e+03 1.35e+03) -1e+02) "0, 0, 0" "1.000000,1.000000,1.000000") "Undefined" 0 0))

(event Custom|EatDestroyed
  (params (DestroyedActor :type Actor%20Object%20Reference))
  (CallFunction|SpawnEat))

(event Custom|SpawnTeleport
  (Game|SpawnActorfromClass "/Game/MyBp/Bp_Teleportator.Bp_Teleportator_C" (Math|Transform|MakeTransform (Math|Vector|MakeVector (Math|Random|RandomFloatinRange -1.35e+03 1.35e+03) (Math|Random|RandomFloatinRange -1.35e+03 1.35e+03) -1e+02) "0, 0, 0" "1.000000,1.000000,1.000000") "Undefined" 0 0))

(event EventBeginPlay
  (CallFunction|SpawnEat)
  (Utilities|Time|SetTimerbyEvent (delegate Custom|Spawn%20Haste) 5.0 true)
  (Utilities|Time|SetTimerbyEvent (delegate Custom|SpawnTeleport) 6e+01 true))

(fn ConstructionScript)